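; Arrows item for the soldier's inventory system, built on a parent item class and purchasable with gold.
; IsBought runs the parent logic, then, if the game instance holds enough gold, deducts the cost and adds one item to the player's InventoryComponent.
; Gold is deducted before the add, whose result is returned.
; UseItem only forwards to the parent, and the event graph is inactive.
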(fn `IsBought`
  (returns (Success :type Boolean))
  (bind _asmy_game_instance (cast `/Game/Character/MyGameInstance` (`GameplayStatics.GetGameInstance`) :!pure true))
  (bind _goldcoinsgi (`/Game/Character/MyGameInstance.GoldCoinsGI` _asmy_game_instance))
  ;[1 1 1] Buys item
  (`parent.IsBought`)
  (if (>= _goldcoinsgi 1)
    (set `/Game/Character/MyGameInstance.GoldCoinsGI` (- _goldcoinsgi 1) _asmy_game_instance)
    (bind _newparam (`/Game/Character/Soldier/InventorySystem/InventoryComponent.AddToInv` (`self.GetComponentByClass` (`GameplayStatics.GetPlayerCharacter` 0) "/Game/Character/Soldier/InventorySystem/InventoryComponent.InventoryComponent_C") (make `/Game/Character/Soldier/InventorySystem/SlotStructure` (`self.ItemStructure`) 1)))
    (return _newparam)))

(fn `UseItem`
  (returns (Success :type Boolean))
  (bind _success (`parent.UseItem`))
  (return _success))

(fn `UserConstructionScript`
  (`parent.UserConstructionScript`))