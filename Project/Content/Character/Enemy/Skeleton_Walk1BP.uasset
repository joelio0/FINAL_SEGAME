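; Walking skeleton enemy for a Paper2D game that patrols back and forth between two points.
; The construction script turns PointA and PointB into relative InterpToMovement control points, and each reversal flips the flipbook's rotation through a FlipFlop.
; Contact damage is inactive: the HitBox overlap only casts to Soldier, with DecreaseHealth unconnected.
; DecreaseHealth itself only casts the player to Soldier, leaving its health subtraction unwired.
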(event `self.InterpToMovement.OnInterpToReverse`
  (params (ImpactResult :type "HitResult Structure (by ref)") (Time :type "Float (single-precision)"))
  (bind _paperflipbook (`self.PaperFlipbook`))
  ;[1 1 1] Movement
  (`/Engine/EditorBlueprintResources/StandardMacros.FlipFlop`
    (:`A`
      (`SceneComponent.K2_SetWorldRotation` _paperflipbook (struct :`Yaw` 180.0) false false))
    (:`B`
      (`SceneComponent.K2_SetWorldRotation` :`self` _paperflipbook))))

(event `self.HitBox.OnComponentBeginOverlap`
  (params (OverlappedComponent :type "PrimitiveComponent Object Reference") (OtherActor :type "Actor Object Reference") (OtherComp :type "PrimitiveComponent Object Reference") (OtherBodyIndex :type Integer) (bFromSweep :type Boolean) (SweepResult :type "HitResult Structure (by ref)"))
  ;[1 1 1] Damage
  (cast `/Game/Character/Soldier/Soldier` OtherActor))

(fn `Decrease Health`
  ;[1 1 1] Decrease Health
  (bind _assoldier (cast `/Game/Character/Soldier/Soldier` (`GameplayStatics.GetPlayerCharacter` 0))))

(fn `UserConstructionScript`
  ;[1 1 1] The ping pong
  (set `InterpToMovementComponent.ControlPoints` (`|MakeArray` (make `InterpControlPoint` (`self.PointA`)) (make `InterpControlPoint` (`self.PointB`))) (`self.InterpToMovement`)))